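; RTS player controller that sets up Enhanced Input, the mouse cursor and the main UI widget.
; Input drives the camera pawn's movement component for move, speed boost, edge scroll, zoom and resets, with a gate enabling mouse panning while suspending edge scroll.
; Each tick, a cursor trace scaled by camera arm length feeds BuildingManager, whose Barracks preview toggles and rotates by key.
; Events relay date-time and game speed to UI and GameState.
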(event Input|EnhancedActionEvents|EnhancedInputActionIA_Move
  (params (ActionValue :type Vector%202D%20Structure) (ElapsedSeconds :type Float%20%28double-precision%29) (TriggeredSeconds :type Float%20%28double-precision%29) (InputAction :type Input%20Action%20Object%20Reference :default "/Game/Core/Player/Inputs/IA_Move.IA_Move"))
  ;[1 1 1] Movement Events
  ;;[1 1 1] WASD Movements
  (Default|BasicMovementControls (Variables|References|GetCameraMovementRef) (.x ActionValue) (.y ActionValue)))

(event Input|EnhancedActionEvents|EnhancedInputActionIA_SpeedModifier
  (params (ActionValue :type Boolean) (ElapsedSeconds :type Float%20%28double-precision%29) (TriggeredSeconds :type Float%20%28double-precision%29) (InputAction :type Input%20Action%20Object%20Reference :default "/Game/Core/Player/Inputs/IA_SpeedModifier.IA_SpeedModifier"))
  (bind _cameramovementref (Variables|References|GetCameraMovementRef))
  ;[1 1 1] Movement Events
  ;;[1 1 1] Call Movement Speed Modifier
  (:Triggered
    (Default|SetSpeedModifier _cameramovementref 2.0))
  (:Canceled
    (Default|SetSpeedModifier _cameramovementref 1.0 :!label _label))
  (:Completed
    (goto _label)))

(event Input|EnhancedActionEvents|EnhancedInputActionIA_ZoomIn
  (params (ActionValue :type Boolean) (ElapsedSeconds :type Float%20%28double-precision%29) (TriggeredSeconds :type Float%20%28double-precision%29) (InputAction :type Input%20Action%20Object%20Reference :default "/Game/Core/Player/Inputs/IA_ZoomIn.IA_ZoomIn"))
  ;[1 1 1] Zoom Events
  ;;[1 1 1] Zoom In / Out
  (Default|Zoomin (Variables|References|GetCameraMovementRef)))

(event Input|EnhancedActionEvents|EnhancedInputActionIA_ZoomOut
  (params (ActionValue :type Boolean) (ElapsedSeconds :type Float%20%28double-precision%29) (TriggeredSeconds :type Float%20%28double-precision%29) (InputAction :type Input%20Action%20Object%20Reference :default "/Game/Core/Player/Inputs/IA_ZoomOut.IA_ZoomOut"))
  ;[1 1 1] Zoom Events
  ;;[1 1 1] Zoom In / Out
  (Default|ZoomOut (Variables|References|GetCameraMovementRef)))

(event Input|EnhancedActionEvents|EnhancedInputActionIA_ZoomReset
  (params (ActionValue :type Boolean) (ElapsedSeconds :type Float%20%28double-precision%29) (TriggeredSeconds :type Float%20%28double-precision%29) (InputAction :type Input%20Action%20Object%20Reference :default "/Game/Core/Player/Inputs/IA_ZoomReset.IA_ZoomReset"))
  ;[1 1 1] Zoom Events
  ;;[1 1 1] Reset Zoom
  (:Started
    (Default|ResetZoom (Variables|References|GetCameraMovementRef))))

(event Input|EnhancedActionEvents|EnhancedInputActionIA_ResetCamera
  (params (ActionValue :type Boolean) (ElapsedSeconds :type Float%20%28double-precision%29) (TriggeredSeconds :type Float%20%28double-precision%29) (InputAction :type Input%20Action%20Object%20Reference :default "/Game/Core/Player/Inputs/IA_ResetCamera.IA_ResetCamera"))
  ;[1 1 1] Reset Camera
  (:Started
    (Default|ResetCamera (Variables|References|GetCameraMovementRef))))

(event Input|EnhancedActionEvents|EnhancedInputActionIA_PanReset
  (params (ActionValue :type Boolean) (ElapsedSeconds :type Float%20%28double-precision%29) (TriggeredSeconds :type Float%20%28double-precision%29) (InputAction :type Input%20Action%20Object%20Reference :default "/Game/Core/Player/Inputs/IA_PanReset.IA_PanReset"))
  ;[1 1 1] Pan Events
  ;;[1 1 1] Reset Pan
  (:Started
    (Default|ResetPan (Variables|References|GetCameraMovementRef))))

(event Input|EnhancedActionEvents|EnhancedInputActionIA_Pan
  (params (ActionValue :type Boolean) (ElapsedSeconds :type Float%20%28double-precision%29) (TriggeredSeconds :type Float%20%28double-precision%29) (InputAction :type Input%20Action%20Object%20Reference :default "/Game/Core/Player/Inputs/IA_Pan.IA_Pan"))
  (bind _cameramovementref (Variables|References|GetCameraMovementRef))
  ;[1 1 1] Pan Events
  ;;[1 1 1] Pan
  (:Triggered
    (Default|SetDisableEdgeScroll _cameramovementref true)
    (Utilities|FlowControl|Gate true) ; enters at Open
  )
  (:Canceled
    (Default|SetDisableEdgeScroll _cameramovementref false :!label _label)
    (Utilities|FlowControl|Gate true) ; enters at Close
  )
  (:Completed
    (goto _label)))

(event Input|EnhancedActionEvents|EnhancedInputActionIA_RotatePreview
  (params (ActionValue :type Float%20%28double-precision%29) (ElapsedSeconds :type Float%20%28double-precision%29) (TriggeredSeconds :type Float%20%28double-precision%29) (InputAction :type Input%20Action%20Object%20Reference :default "/Game/Core/Player/Inputs/IA_RotatePreview.IA_RotatePreview"))
  (bind _buildingmanager (Variables|Default|GetBuildingManager))
  (:Started
    (switch int (Math|Float|Truncate ActionValue)
      (:-1
        (Default|RotatePreviewLeft _buildingmanager))
      (:1
        (Default|RotatePreviewRight _buildingmanager)))))

(event EventBeginPlay
  (Utilities|FlowControl|Sequence
    (:then_0
      (Input|AddMappingContext (PlayerController|LocalPlayerSubsystems|GetEnhancedInputLocalPlayerSubsystem) "/Game/Core/Player/Inputs/IMC_RTS.IMC_RTS" 0 "(bIgnoreAllPressedKeysUntilRelease=True,bForceImmediately=False,bNotifyUserSettings=False)")
      (Variables|Default|SetbShowMouseCursor true)
      (bind _asbp_camera_pawn (Utilities|Casting|CastToBP_CameraPawn (Game|Player|GetPlayerPawn 0)))
      (bind _output_get (Variables|References|SetCameraPawnRef _asbp_camera_pawn))
      (Variables|References|SetCameraMovementRef (Variables|/Game/Core/Player/BP_CameraPawn.BP_CameraPawn_C|GetPawnMovementComponent _output_get)))
    (:then_1
      (bind _returnvalue (UserInterface|CreateWidget "/Game/Core/Widgets/WDP_MainUI.WDP_MainUI_C" self))
      (bind _output_get_2 (Variables|References|SetMainWidgetRef _returnvalue))
      (UserInterface|Viewport|AddtoViewport _output_get_2 0)
      (Input|SetInputModeGameandUI self _output_get_2 "LockInFullscreen" false false))))

(event EventTick
  (params (DeltaSeconds :type Float%20%28single-precision%29))
  (bind _output_get (Variables|DoNotdEdit|SetMousePosition (CallFunction|SetMousePosition (+ (Default|GetCurrentArmLength (Variables|References|GetCameraPawnRef)) 2e+03))))
  (Default|SetMousePosition (Variables|Default|GetBuildingManager) _output_get))

(event EventSetDateTime
  (params (DateTimeStruct :type Date%20Time%20Structure))
  (Class|BPIGameTime|SetDateTime(Message) (Variables|References|GetMainWidgetRef) DateTimeStruct))

(event EventUpdateGameSpeed
  (params (NewSpeedMultiplier :type Float%20%28double-precision%29))
  (Class|BPIGameTime|UpdateGameSpeed(Message) (Game|GetGameState) NewSpeedMultiplier))

(event EventSetGameSpeedInt
  (params (GameSpeed :type Float%20%28double-precision%29))
  (Class|BPIGameTime|SetGameSpeedInt(Message) (Variables|References|GetMainWidgetRef) GameSpeed))

(event Input|MouseEvents|MouseX
  (params (AxisValue :type Float%20%28single-precision%29))
  ;[1 1 1] Pan Events
  ;;[1 1 1] Pan
  (Utilities|FlowControl|Gate true
    (:Exit
      (Default|PanCamera (Variables|References|GetCameraMovementRef) (* AxisValue (Variables|Camera|Settings|GetPanSensitivity))))))

(event Input|MouseEvents|MouseX
  (params (AxisValue :type Float%20%28single-precision%29))
  ;[1 1 1] Movement Events
  ;;[1 1 1] Edge Scroll
  (Default|EdgeScroll (Variables|References|GetCameraMovementRef)))

(event Input|MouseEvents|MouseY
  (params (AxisValue :type Float%20%28single-precision%29))
  ;[1 1 1] Movement Events
  ;;[1 1 1] Edge Scroll
  (Default|EdgeScroll (Variables|References|GetCameraMovementRef)))

(event Input|KeyboardEvents|B
  (params (Key :type Key%20Structure :default "None"))
  (bind _buildingmanager (Variables|Default|GetBuildingManager))
  (:Pressed
    (Utilities|FlowControl|FlipFlop
      (:A
        (Default|SetPreview _buildingmanager "Barracks"))
      (:B
        (Default|DestroyPreview _buildingmanager)))))

(fn ConstructionScript)

(fn SetMousePosition
  (params (TraceDIstance :type Float%20%28double-precision%29))
  (bind (_worldlocation _worlddirection) (Game|Player|ConvertMouseLocationToWorldSpace))
  (bind _outhit (Collision|LineTraceByChannel _worldlocation (+ _worldlocation (* _worlddirection TraceDIstance)) "TraceTypeQuery3" false 0 "None"))
  (if (!= (.HitActor (Collision|BreakHitResult _outhit)) 0)
    (return (.Location (Collision|BreakHitResult _outhit)))))